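; BP_Cube is an object that exercises JSON-based save and load hooks with test data.
; OnSave writes a fixed test string field into the JsonObject, and OnLoad reads it back, printing a message with the object's name when the value matches.
; OnPostLoad prints a debug message, and the construction script is empty.
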(event `self.OnLoad`
  (params (JsonObject :type "JSONLibrary Object Reference"))
  (bind (_stringvalue _returnvalue) (`JSONLibrary.GetValueAsString` JsonObject "TestField"))
  (if _returnvalue
    (if (`KismetStringLibrary.EqualEqual_StrStr` _stringvalue "SomeData")
      (`KismetSystemLibrary.PrintString` (`KismetStringLibrary.Concat_StrStr` "Loaded String Data from " (`KismetSystemLibrary.GetObjectName` self))))))

(event `self.OnPostLoad`
  (`KismetSystemLibrary.PrintString` "PostLoad" true true (struct :`G` 0.66 :`B` 1.0 :`A` 1.0) 5.0))

(event `self.OnSave`
  (params (JsonObject :type "JSONLibrary Object Reference"))
  (`JSONLibrary.SetValueAsString` JsonObject "TestField" "SomeData"))

(fn `UserConstructionScript`)